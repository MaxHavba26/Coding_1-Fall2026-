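; BP_Spawner is an actor that spawns instances of a configurable class at its SpawnPoint component.
; With AutoSpawn on, BeginPlay prints a message and calls the SpawnThings event, which re-calls itself after a fixed Delay to form a repeating loop.
; SpawnThings performs a single spawn when AutoSpawn is off, and every spawn is skipped if it would collide.
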(event `self.ReceiveBeginPlay`
  (if (`self.AutoSpawn?`)
    (`KismetSystemLibrary.PrintText` "Spawn actives")
    (`self.Spawn Things`)))

(event `Spawn Things`
  (`|SpawnActorFromClass` (`self.SpawnPointer`) (`SceneComponent.K2_GetComponentToWorld` (`self.SpawnPoint`)) "DontSpawnIfColliding" "MultiplyWithRoot" null null)
  (if (`self.AutoSpawn?`)
    (`KismetSystemLibrary.Delay` 5.0)
    (`self.Spawn Things`)))

(fn `UserConstructionScript`)