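; BP_TreeManager is a manager that animates the level's BP_Tree actors, gathering them into an array shortly after BeginPlay.
; ShiftLeaves randomly rescales child components in a loop and re-calls itself through a short Delay to keep them changing.
; HideTrees hides every gathered tree, then ShowTrees reveals them one per second by calling itself with an incrementing index until the array ends.
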(event `self.ReceiveBeginPlay`
  (`KismetSystemLibrary.PrintText` "Tree manager startin")
  (`KismetSystemLibrary.Delay` 3.0)
  (bind _outactors (`GameplayStatics.GetAllActorsOfClass` "/Game/Coding1/Blueprints/BP_Tree.BP_Tree_C"))
  (set `self.Tree Array` _outactors)
  (`self.ShiftLeaves`)
  (`self.HideTrees`)
  (`self.ShowTrees`))

(event `ShiftLeaves`
  (for _array_element _
    (for _array_element_2 (`SceneComponent.GetChildrenComponents` _array_element true)
      (`SceneComponent.SetRelativeScale3D` _array_element_2 (* (1.0 1.0 1.0) (`KismetMathLibrary.RandomFloatInRange` 0.6 4.0)))
      (`KismetSystemLibrary.Delay` 0.2)
      (`self.ShiftLeaves`))))

(event `HideTrees`
  (for _array_element (`self.Tree Array`)
    (`self.SetActorHiddenInGame` _array_element true)))

(event `ShowTrees`
  (bind _index (`self.Index`))
  (bind _tree_array (`self.Tree Array`))
  (`KismetSystemLibrary.Delay` 1.0)
  (`self.SetActorHiddenInGame` (`|GetArrayItem` _tree_array _index) false)
  (bind _result (`/Engine/EditorBlueprintResources/StandardMacros.IncrementInt` _index)
    (:`  `
      (if (not (== _result (`KismetArrayLibrary.Array_Length` _tree_array)))
        (`self.ShowTrees`)))))

(fn `UserConstructionScript`)