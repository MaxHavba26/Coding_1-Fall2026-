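; Spawn manager that periodically triggers the level's BP_Spawner actors, one at a time.
; On BeginPlay it gathers every spawner, then a self-calling event with a fixed delay steps through the list, calling SpawnThings only on those without AutoSpawn.
; When the index passes the end, the list is reshuffled and restarted, so each later pass visits every spawner once in random order.
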(event `self.ReceiveBeginPlay`
  (bind _outactors (`GameplayStatics.GetAllActorsOfClass` "/Game/Coding1/Blueprints/BP_Spawner.BP_Spawner_C"))
  (set `self.Spawners` _outactors)
  (`self.Spawn Permission`))

(event `Spawn Permission`
  (bind _spawners (`self.Spawners`))
  (bind _index (`self.Index`))
  (bind _output (`|GetArrayItem` (`self.Spawners`) _index))
  (if (>= (`self.Index`) (`KismetArrayLibrary.Array_Length` _spawners))
    ; reshuffle spawners and reset the index
    (`KismetArrayLibrary.Array_Shuffle` _spawners)
    (set `self.Index` 0))
  (if (not (`/Game/Coding1/Blueprints/BP_Spawner.AutoSpawn?` _output))
    (`/Game/Coding1/Blueprints/BP_Spawner.Spawn Things` _output))
  (`/Engine/EditorBlueprintResources/StandardMacros.IncrementInt` _index
    (:`  `
      (`KismetSystemLibrary.Delay` 5.0)
      (`self.Spawn Permission`))))

(fn `UserConstructionScript`)